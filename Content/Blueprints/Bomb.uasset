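; Bomb actor that swells on a timeline after BeginPlay and explodes after a short fuse timer.
; Explode spawns four ExplosionProjectiles at right angles, with lifespan scaled by BombStrength to set blast reach, then plays a sound and destroys the bomb.
; Ending an overlap fires CallLeftBombCollision.
; An unconnected multi-line trace that destroys hit actors never runs.
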(event Custom|Explode
  (for _index (range 0 3)
    (bind _returnvalue (Game|SpawnActorfromClass "/Game/Blueprints/ExplosionProjectile.ExplosionProjectile_C" (Math|Transform|MakeTransform (+ (Transformation|GetActorLocation) "0.000000,0.000000,100.000000") (Math|Conversions|RotationFromXVector (Math|Vector|RotateVector "1.000000,0.000000,0.000000" (Math|Rotator|MakeRotator 0.0 0.0 (Math|Conversions|ToFloat(Integer) (* _index 90))))) "1.000000,1.000000,1.000000") "Undefined" "MultiplyWithRoot" 0 0))
    (Actor|SetLifeSpan _returnvalue (* (Variables|Default|GetBombStrength) 0.1)))
  (Audio|PlaySoundatLocation "/Game/Audio/kaboom.kaboom" (Transformation|GetActorLocation) "0, 0, 0" 1.0 1.0 0.0 0 0 0 0)
  (Actor|DestroyActor))

(event EventBeginPlay
  (Utilities|Time|SetTimerbyEvent (delegate Custom|Explode) 3.0)
  (bind _bombscale (Timeline|ExplodingTL Play)
    (:Update
      (Transformation|SetWorldScale3D (Variables|Default|GetStaticMesh) (Math|Conversions|ToVector(Float) _bombscale)))))

(event Collision|EventActorEndOverlap
  (params (OtherActor :type Actor%20Object%20Reference))
  (Default|CallLeftBombCollision))

(fn ConstructionScript)