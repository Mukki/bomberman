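; Player knight character for a grid-based bomb-planting game, moved along world X and Y axes by MoveUp and MoveRight inputs.
; PlantBomb spawns a Bomb owned by the knight at its location snapped to a 200-unit grid.
; The capsule ignores the new bomb's BlockBox while moving, then clears all move-ignores when the bomb's LeftBombCollision event fires, letting the knight step off it.
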(event Custom|ClearBombCollision
  (Class|PrimitiveComponent|ClearMoveIgnoreComponents (Variables|Collision|GetCapsuleComponent)))

(event EventBeginPlay)

(event Collision|EventActorBeginOverlap
  (params (OtherActor :type Actor%20Object%20Reference)))

(event EventTick
  (params (DeltaSeconds :type Float%20%28single-precision%29)))

(event Input|ActionEvents|InputActionPlantBomb
  (params (Key :type Key%20Structure :default "None"))
  (:Pressed
    (bind _returnvalue (Game|SpawnActorfromClass "/Game/Blueprints/Bomb.Bomb_C" (Math|Transform|MakeTransform (Class|KismetMathLibrary|VectorSnappedtoGrid (Transformation|GetActorLocation) 2e+02) "0, 0, 0" "1.000000,1.000000,1.000000") "AlwaysSpawn" "MultiplyWithRoot" self 0))
    (Class|PrimitiveComponent|IgnoreComponentwhenMoving (Variables|Collision|GetCapsuleComponent) (Variables|/Game/Blueprints/Bomb.Bomb_C|GetBlockBox _returnvalue) true)
    (EventDispatchers|BindEventtoLeftBombCollision _returnvalue (delegate Custom|ClearBombCollision))))

(event Input|AxisEvents|InputAxisMoveUp
  (params (AxisValue :type Float%20%28single-precision%29))
  (Pawn|Input|AddMovementInput "1.000000,0.000000,0.000000" AxisValue false))

(event Input|AxisEvents|InputAxisMoveRight
  (params (AxisValue :type Float%20%28single-precision%29))
  (Pawn|Input|AddMovementInput "0.000000,1.000000,0.000000" AxisValue false))

(fn ConstructionScript)