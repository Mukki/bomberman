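; BarbarianCharacter is a playable character that moves along world X and Y axes and plants bombs, in a Bomberman-like style.
; PlantBomb spawns a Bomb at the character's grid-snapped location, passing its current BombStrength.
; The capsule ignores the new bomb's BlockBox while moving until the bomb's left-collision event clears all move ignores.
; Separate events raise BombStrength within a clamped range and set ShieldHP.
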(event Custom|SetShieldHP
  (params (HP :type Integer64))
  (Variables|Default|SetShield%20HP HP))

(event Custom|ClearBombCollision
  (Class|PrimitiveComponent|ClearMoveIgnoreComponents (Variables|Collision|GetCapsuleComponent)))

(event Custom|IncreaseBombStrength
  (Variables|Default|SetBomb%20Strength (Math|Integer|Clamp(Integer) (+ (Variables|Default|GetBomb%20Strength) 1) 0 10)))

(event EventBeginPlay)

(event Collision|EventActorBeginOverlap
  (params (OtherActor :type Actor%20Object%20Reference)))

(event EventTick
  (params (DeltaSeconds :type Float%20%28single-precision%29)))

(event Input|ActionEvents|InputActionPlantBomb
  (params (Key :type Key%20Structure :default "None"))
  (:Pressed
    (bind _returnvalue (Game|SpawnActorfromClass "/Game/Blueprints/Bomb.Bomb_C" (Math|Transform|MakeTransform (Class|KismetMathLibrary|VectorSnappedtoGrid (Transformation|GetActorLocation) 2e+02) "0, 0, 0" "1.000000,1.000000,1.000000") "AlwaysSpawn" "MultiplyWithRoot" self (Variables|Default|GetBomb%20Strength) 0))
    (Class|PrimitiveComponent|IgnoreComponentwhenMoving (Variables|Collision|GetCapsuleComponent) (Variables|/Game/Blueprints/Bomb.Bomb_C|GetBlockBox _returnvalue) true)
    (EventDispatchers|BindEventtoLeftBombCollision _returnvalue (delegate Custom|ClearBombCollision))))

(event Input|AxisEvents|InputAxisMoveUp
  (params (AxisValue :type Float%20%28single-precision%29))
  (Pawn|Input|AddMovementInput "1.000000,0.000000,0.000000" AxisValue false))

(event Input|AxisEvents|InputAxisMoveRight
  (params (AxisValue :type Float%20%28single-precision%29))
  (Pawn|Input|AddMovementInput "0.000000,1.000000,0.000000" AxisValue false))

(fn ConstructionScript)