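; Bomberman arena mode Blueprint that randomizes the crate layout when play begins.
; BeginPlay calls GenerateLevel, which gathers every Crate actor already in the level and destroys a random fraction, set here to one fifth.
; Each picked crate is removed from the working array so it cannot be chosen again, and the GameSetup flag is cleared afterwards.
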(event EventBeginPlay
  (CallFunction|GenerateLevel 0.2))

(event EventTick
  (params (DeltaSeconds :type Float%20%28single-precision%29)))

(fn ConstructionScript)

(fn GenerateLevel
  (params (CreateDeletionPercentage :type Float%20%28double-precision%29))
  (bind _outactors (Actor|GetAllActorsOfClass "/Game/Blueprints/Crate.Crate_C"))
  (Variables|Default|SetCrates _outactors)
  (for _index (range 0 (Math|Float|Truncate (* (Utilities|Array|Length _outactors) CreateDeletionPercentage)))
    (bind _output_get (Variables|Default|SetRandomCrate (.OutItem (Utilities|Array|Random (Variables|Default|GetCrates)))))
    (Actor|DestroyActor _output_get)
    (Utilities|Array|RemoveItem (Variables|Default|GetCrates) (Variables|Default|GetRandomCrate)))
  (Variables|Default|SetGameSetup false))