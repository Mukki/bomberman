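; ObjectSpawner is an actor, filed under main menu objects, that continuously spawns short-lived random objects around its location.
; From BeginPlay, SpawnObject picks a class from an array whose duplicate entries weight Object5 and Object6, then spawns it at a random Y offset and rotation.
; Each spawn gets a fixed lifespan, and the event calls itself again after a random short delay.
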(event Custom|SpawnObject
  (bind _returnvalue (Game|SpawnActorfromClass (.OutItem (Utilities|Array|Random (Utilities|Array|MakeArray "/Game/Blueprints/MainMenuObjects/Object1.Object1_C" "/Game/Blueprints/MainMenuObjects/Object2.Object2_C" "/Game/Blueprints/MainMenuObjects/Object3.Object3_C" "/Game/Blueprints/MainMenuObjects/Object4.Object4_C" "/Game/Blueprints/MainMenuObjects/Object5.Object5_C" "/Game/Blueprints/MainMenuObjects/Object6.Object6_C" "/Game/Blueprints/MainMenuObjects/Object5.Object5_C" "/Game/Blueprints/MainMenuObjects/Object5.Object5_C" "/Game/Blueprints/MainMenuObjects/Object6.Object6_C"))) (Math|Transform|MakeTransform (+ (Transformation|GetActorLocation) (Math|Vector|MakeVector 0.0 (Math|Random|RandomFloatinRange -5e+02 5e+02) 0.0)) (Math|Random|RandomRotator false) "1.000000,1.000000,1.000000") "Undefined" "MultiplyWithRoot" 0 0))
  (Actor|SetLifeSpan _returnvalue 5.0)
  (Utilities|FlowControl|Delay (Math|Random|RandomFloatinRange 0.3 1.0))
  (CallFunction|SpawnObject))

(event EventBeginPlay
  (CallFunction|SpawnObject))

(event Collision|EventActorBeginOverlap
  (params (OtherActor :type Actor%20Object%20Reference)))

(event EventTick
  (params (DeltaSeconds :type Float%20%28single-precision%29)))

(fn ConstructionScript)